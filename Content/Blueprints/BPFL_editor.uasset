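; BPFL_editor is a function library of shared helpers for an editor that works with notes, lines and events.
; It reads note separation from the BPGI_editor game instance and shows error popups as top-layer viewport widgets.
; Two Select tables convert between nine consecutive line indices and sparse event IDs up to 13, with unused IDs falling back to line zero.
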(fn `EventToLine`
  (params (Event :type Integer))
  (returns (Line :type Integer))
  (return (select `int` Event :`0` 0 :`1` 1 :`2` 2 :`3` 3 :`4` 4 :`5` 0 :`6` 0 :`7` 0 :`8` 5 :`9` 6 :`10` 0 :`11` 0 :`12` 7 :`13` 8)))

(fn `GetNoteSep`
  (returns (Separation :type "Float (double-precision)"))
  (return (`/Game/Blueprints/BPGI_editor.NoteSeparation` (cast `/Game/Blueprints/BPGI_editor` (`GameplayStatics.GetGameInstance` (`local.__WorldContext`)) :!pure true))))

(fn `LineToEvent`
  (params (Line :type Integer))
  (returns (Event :type Integer))
  (return (select `int` Line :`0` 0 :`1` 1 :`2` 2 :`3` 3 :`4` 4 :`5` 8 :`6` 9 :`7` 12 :`8` 13)))

(fn `SpawnPopup`
  (params (Message :type String))
  (bind _returnvalue (`|CreateWidget` "/Game/Blueprints/WidgetErrorPopup.WidgetErrorPopup_C" (`GameplayStatics.GetPlayerController` null) Message))
  (`UserWidget.AddToViewport` _returnvalue 10000))