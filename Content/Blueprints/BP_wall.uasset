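; BP_wall is a lane-based wall obstacle whose shape is derived from its Line, Width, Duration and Type values.
; UpdateWall scales MeshRoot by lane width, duration as depth, and a Type-selected height, then offsets it sideways to its line and vertically by Type.
; The construction script calls UpdateWall, so the wall takes its shape whenever the actor is constructed.
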(event `UpdateWall`
  (bind _type (`self.Type`))
  (bind _meshroot (`self.MeshRoot`))
  (`SceneComponent.SetWorldScale3D` _meshroot (`KismetMathLibrary.MakeVector` (/ (* (`self.Width`) 70.0) 100.0) (* (`self.Duration`) 2.0) (/ (select `int` _type :`0` 280.0 :`1` 140.0 :!type "Float (single-precision)") 100.0)))
  (`SceneComponent.K2_SetRelativeLocation` _meshroot (`KismetMathLibrary.MakeVector` (* (`self.Line`) 70.0) 0.0 (select `int` _type :`0` -40.0 :`1` 100.0 :!type "Float (single-precision)")) false false))

(fn `UserConstructionScript`
  (`self.UpdateWall`))