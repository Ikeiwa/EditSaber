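; BP_note_ghost is a ghost version of a rhythm-game note, shown as a red or blue cube or a bomb.
; UpdateNote, also run by the construction script, sets mesh and materials by Type, shows a dot or arrow for cubes by Direction, then calls UpdateTransform.
; UpdateTransform pitches the mesh by Direction, offsets NoteRoot onto a Line and Layer grid, and places the actor along negative Y by Time times note separation.
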(event `Update Note`
  (bind _point (`self.Point`))
  (bind _point_2 (`self.Point`))
  (bind _arrow (`self.Arrow`))
  (bind _mesh (`self.Mesh`))
  (`|ExecutionSequence`
    (:`then_0`
      (switch `int` (`self.Type`)
        (:`0`
          (`StaticMeshComponent.SetStaticMesh` _mesh "/Game/Meshes/SM_CubeNote.SM_CubeNote")
          (`PrimitiveComponent.SetMaterial` _mesh 0 "/Game/Materials/M_ghost_note_red.M_ghost_note_red")
          (`PrimitiveComponent.SetMaterial` _point 0 "/Game/Materials/M_Arrow_red.M_Arrow_red")
          (`PrimitiveComponent.SetMaterial` (`self.Arrow`) 0 "/Game/Materials/M_Arrow_red.M_Arrow_red")
          (if (== (`self.Direction`) 8) :!label _label
            (`SceneComponent.SetVisibility` _point_2 true false)
            (`SceneComponent.SetVisibility` _arrow false false)
            (else
              (`SceneComponent.SetVisibility` _point_2 false false)
              (`SceneComponent.SetVisibility` _arrow true false))))
        (:`1`
          (`StaticMeshComponent.SetStaticMesh` _mesh "/Game/Meshes/SM_CubeNote.SM_CubeNote")
          (`PrimitiveComponent.SetMaterial` _mesh 0 "/Game/Materials/M_ghost_note_blue.M_ghost_note_blue")
          (`PrimitiveComponent.SetMaterial` _point 0 "/Game/Materials/M_Arrow_blue.M_Arrow_blue")
          (`PrimitiveComponent.SetMaterial` (`self.Arrow`) 0 "/Game/Materials/M_Arrow_blue.M_Arrow_blue")
          (goto _label))
        (:`3`
          (`StaticMeshComponent.SetStaticMesh` _mesh "/Game/Meshes/SM_Bomb.SM_Bomb")
          (`PrimitiveComponent.SetMaterial` _mesh 0 "/Game/Materials/M_bomb_ghost.M_bomb_ghost")
          (`SceneComponent.SetVisibility` (`self.Point`) false false)
          (`SceneComponent.SetVisibility` (`self.Arrow`) false false))))
    (:`then_1`
      (`self.UpdateTransform`))))

(event `UpdateTransform`
  (`|ExecutionSequence`
    (:`then_0`
      (`SceneComponent.K2_SetRelativeRotation` (`self.Mesh`) (`KismetMathLibrary.MakeRotator` 0.0 (select `int` (`self.Direction`) :`0` 180.0 :`1` 0.0 :`2` 270.0 :`3` 90.0 :`4` 225.0 :`5` 135.0 :`6` 315.0 :`7` 45.0 :`8` 0.0 :!type "Float (single-precision)")) false false))
    (:`then_1`
      (`SceneComponent.K2_SetRelativeLocation` (`self.NoteRoot`) (`KismetMathLibrary.MakeVector` (- (* (`self.Line`) 70.0) 105.0) 0.0 (* (`self.Layer`) 70.0)) false false)
      (`self.K2_SetActorRelativeLocation` (`KismetMathLibrary.MakeVector` 0.0 (* (* (`/Game/Blueprints/BPFL_editor.GetNoteSep`) (`self.Time`)) -1.0))))))

(fn `UserConstructionScript`
  (`self.Update Note`))